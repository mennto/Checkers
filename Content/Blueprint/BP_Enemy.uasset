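; BP_Enemy is an unfinished opponent for a checkers game, meant to play the black side.
; On every Tick while the board reference RefDesk has TurnWalk false, it scans the Field for valid pieces with a false SIdeColor.
; It writes those pieces into AviableCheckers at a running Index, which is never reset here.
; MakeMove is an empty stub whose only call is unreachable, so no move is made.
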(event `self.ReceiveTick`
  (params (DeltaSeconds :type "Float (single-precision)"))
  (if (not (`/Game/Blueprint/BP_Desk.Turn Walk` (`self.Ref_Desk`)))
    (`self.Found Black Checker`)))

(fn `Found Black Checker`
  (for _array_element (`/Game/Blueprint/BP_Desk.Field` (`self.Ref_Desk`))
    (`/Engine/EditorBlueprintResources/StandardMacros.IsValid` _array_element
      (:`Is Valid`
        (if (not (`/Game/Blueprint/BP_Checker.SIde(color)` _array_element))
          (`KismetArrayLibrary.Array_Set` (`self.Aviable Checkers`) (`self.Index`) _array_element)
          (bind _result (`/Engine/EditorBlueprintResources/StandardMacros.IncrementInt` (`self.Index`))
            (:`  `
              (set `self.Index` _result))))))))

(fn `Make Move`
  (params (Coordinate :type Integer)))

(fn `UserConstructionScript`)