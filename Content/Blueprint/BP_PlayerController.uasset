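; Player controller that builds a checkers game on BeginPlay, spawning a desk and populating it with pieces.
; A loop over the 8x8 grid uses IdentifyCell to pass only alternating squares outside the two middle rows.
; Each passing index spawns a checker at its grid position, sets material, side and movement direction by board half, links it to the desk and stores it in the desk's Field array.
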(event `self.ReceiveBeginPlay`
  (`self.Spawn Desk`)
  (for _index (range 64)
    (`self.IdentifyCell` _index)
    (bind _checker (`self.Spawn Checker` _index))
    (`self.SetCheckerParam` _checker _index)
    (`KismetArrayLibrary.Array_Set` (`/Game/Blueprint/BP_Desk.Field` (`self.Ref_Desk`)) _index _checker)))

(fn `SetCheckerParam`
  (params (Checher :type "/Game/Blueprint/BP_Checker Object Reference") (Index :type Integer))
  (bind _ref_desk (`self.Ref_Desk`))
  (bind _index (`local.Index`))
  (bind _staticmesh (`/Game/Blueprint/BP_Checker.StaticMesh` Checher))
  (if (>= Index 31)
    (`PrimitiveComponent.SetMaterial` _staticmesh 0 "/Game/Material/M_black.M_black")
    (set `/Game/Blueprint/BP_Checker.SIde(color)` false Checher)
    (set `/Game/Blueprint/BP_Checker.X_Offset` -1 Checher)
    (set `/Game/Blueprint/BP_Checker.Posithion` _index Checher)
    (set `/Game/Blueprint/BP_Checker.Ref_Desk` _ref_desk Checher)
    (else
      (`PrimitiveComponent.SetMaterial` _staticmesh 0 "/Game/Material/M_white.M_white")
      (set `/Game/Blueprint/BP_Checker.SIde(color)` true Checher)
      (set `/Game/Blueprint/BP_Checker.X_Offset` 1 Checher)
      (set `/Game/Blueprint/BP_Checker.Posithion` _index Checher)
      (set `/Game/Blueprint/BP_Checker.Ref_Desk` _ref_desk Checher))))

(fn `Spawn Checker`
  (params (Index :type Integer))
  (returns (Checker :type "/Game/Blueprint/BP_Checker Object Reference"))
  (bind _returnvalue (`|SpawnActorFromClass` "/Game/Blueprint/BP_Checker.BP_Checker_C" (`KismetMathLibrary.Conv_VectorToTransform` (`KismetMathLibrary.MakeVector` (+ (* (/ Index 8) 50.0) 25.0) (+ (* (mod Index 8) 50.0) 25.0) 32.0)) "Undefined" "OverrideRootScale" null null))
  (return _returnvalue))

(fn `Spawn Desk`
  (bind _returnvalue (`|SpawnActorFromClass` "/Game/Blueprint/BP_Desk.BP_Desk_C" (`KismetMathLibrary.Conv_VectorToTransform` (200.0 200.0 20.0)) "Undefined" "OverrideRootScale" null null))
  (set `self.Ref_Desk` _returnvalue))

(fn `UserConstructionScript`)