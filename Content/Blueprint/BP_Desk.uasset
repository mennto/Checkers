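; Checkers board actor that runs a two-sided match, covering moves, mandatory captures, multi-jumps, queen promotion, HUD kill counts and the end screen at twelve kills.
; Pieces live in a flat 64-slot Field, with helpers converting indices to grid coordinates and flipping direction buffers to scan diagonals.
; IdentifyWays, AddPoint and QueenWays fill each piece's possible moves.
; Board clicks match the cursor hit to those moves, then move, capture and switch turns.
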(event `self.ReceiveBeginPlay`
  (`self.Create HUD`)
  (for _ (range 64)
    (`KismetArrayLibrary.Array_Add` (`self.Field`))))

(event `self.ReceiveActorOnClicked`
  (params (ButtonPressed :type "Key Structure"))
  (bind _posibleways (`/Game/Blueprint/BP_Checker.PosibleWays` (`self.Ref_Checker`)))
  (`self.Set Input Coordinates`)
  (if (`self.IsClick`)
    (for _index (range 64)
      (`self.Set Clicked Checker` _index))
    (if (== (`KismetArrayLibrary.Array_Length` _posibleways) 0)
      (`self.Reset Checkers` null)
      (else
        (for _array_element _posibleways
          (`self.Set Clicked Point` _array_element))
        (if (> (`self.Clicked_Point`) -1)
          (`self.Move`)
          (if (`self.Probably Streak`)
            (set `self.Clicked_Point` -1)
            (else
              (`self.Reset Checkers` null :!label _label)
              (set `self.Under Attack` false)
              (set `self.Clicked_Point` -1)
              (`self.IsEnded`)))
          (elif (not (`self.Probably Streak`))
            (goto _label)))))))

(event `self.StaticMesh.OnBeginCursorOver`
  (params (TouchedComponent :type "PrimitiveComponent Object Reference"))
  (set `PlayerController.CurrentMouseCursor` "Crosshairs" (`GameplayStatics.GetPlayerController` 0)))

(event `self.StaticMesh.OnEndCursorOver`
  (params (TouchedComponent :type "PrimitiveComponent Object Reference"))
  (set `PlayerController.CurrentMouseCursor` "Default" (`GameplayStatics.GetPlayerController` 0)))

(fn `Add Point`
  (params (Checker :type "/Game/Blueprint/BP_Checker Object Reference"))
  (bind _checker (`local.Checker`))
  (bind _probably_streak (`self.Probably Streak`))
  (`|ExecutionSequence`
    (:`then_0`
      (for _index (range 4)
        (if (`self.Multiplicity2` _index)
          (`self.Change_Buf_Variables` :!label _label
            (:`Output`
              (bind (_new_index _real) (`self.New Point` (`/Game/Blueprint/BP_Checker.Posithion` (`local.Checker`)) (`self.buf_X`) (`self.buf_Y`)))
              (if _real
                (bind _output (`|GetArrayItem` (`self.Field`) _new_index))
                (`/Engine/EditorBlueprintResources/StandardMacros.IsValid` _output
                  (:`Is Valid`
                    (if (`self.Is_Enemy` (`local.Checker`) _output)
                      (bind (_new_index_2 _real_2) (`self.New Point` _new_index (`self.buf_X`) (`self.buf_Y`)))
                      (if _real_2
                        (`/Engine/EditorBlueprintResources/StandardMacros.IsValid` (`|GetArrayItem` (`self.Field`) _new_index_2)
                          (:`Is Not Valid`
                            (`KismetArrayLibrary.Array_Add` (`/Game/Blueprint/BP_Checker.PosibleWays` (`local.Checker`)) _new_index_2))))))))))
          (else
            (goto _label :!via `False`)))))
    (:`then_1`
      (if (== (`KismetArrayLibrary.Array_Length` (`/Game/Blueprint/BP_Checker.PosibleWays` Checker)) 0)
        (if _probably_streak
          (set `self.Probably Streak` false)
          (set `/Game/Blueprint/BP_Checker.Streak` false (`self.Ref_Checker`))
          (else
            (for _ (range 2)
              (set `self.buf_Y` (* (`self.buf_Y`) -1))
              (bind (_new_index_3 _real_3) (`self.New Point` (`/Game/Blueprint/BP_Checker.Posithion` _checker) (`/Game/Blueprint/BP_Checker.X_Offset` _checker) (`self.buf_Y`)))
              (if _real_3
                (`/Engine/EditorBlueprintResources/StandardMacros.IsValid` (`|GetArrayItem` (`self.Field`) _new_index_3)
                  (:`Is Not Valid`
                    (`KismetArrayLibrary.Array_Add` (`/Game/Blueprint/BP_Checker.PosibleWays` (`local.Checker`)) _new_index_3)))))))
        (elif _probably_streak
          (set `/Game/Blueprint/BP_Checker.Streak` true (`self.Ref_Checker`))
          (else
            (set `self.Under Attack` true)
            (set `/Game/Blueprint/BP_Checker.Attack` true (`local.Checker`))))))))

(fn `Create HUD`
  (bind _returnvalue (`|CreateWidget` "/Game/Blueprint/WBP_HUD.WBP_HUD_C"))
  (`/Engine/EditorBlueprintResources/StandardMacros.IsValid` _returnvalue
    (:`Is Valid`
      (`UserWidget.AddToViewport` _returnvalue 0)
      (set `self.Ref_HUD` _returnvalue)
      (`self.Update Text`))))

(fn `Identify Ways`
  (for _array_element (`self.Field`)
    (`/Engine/EditorBlueprintResources/StandardMacros.IsValid` _array_element
      (:`Is Valid`
        (if (== (`self.Turn Walk`) (`/Game/Blueprint/BP_Checker.SIde(color)` _array_element))
          (if (`/Game/Blueprint/BP_Checker.Is Queen` _array_element)
            (`self.Queen Ways` _array_element)
            (else
              (`self.Add Point` _array_element))))))))

(fn `IsEnded`
  (if (or (== (`self.White Kills`) 12) (== 12 (`self.Black Kills`)))
    (`self.Set Winner`)
    (bind _returnvalue (`|CreateWidget` "/Game/Blueprint/WBP_EndGame.WBP_EndGame_C"))
    (`UserWidget.AddToViewport` _returnvalue 0)
    (`TextBlock.SetText` (`/Game/Blueprint/WBP_EndGame.Winner` _returnvalue) (`self.Win`))))

(fn `Killed Posithion`
  (params (`Clicked Posithion` :type Integer) (`Checker Posithion` :type Integer))
  (returns (`Killed Posithion` :type Integer))
  (locals (Killed :type Integer) (Decrement :type Integer))
  (bind _returnvalue (- `Clicked Posithion` `Checker Posithion`))
  (if (> _returnvalue 0)
    (set `local.Decrement` -1)
    (else
      (set `local.Decrement` 1)))
  (if (== (mod _returnvalue 7) 0)
    (set `local.Killed` (+ (`local.Checker Posithion`) (* (+ (/ _returnvalue 7) (`local.Decrement`)) 7)))
    (else
      (set `local.Killed` (+ (`local.Checker Posithion`) (* (+ (/ _returnvalue 9) (`local.Decrement`)) 9)))))
  (return (`local.Killed`)))

(fn `New Point`
  (params (Index :type Integer) (X :type Integer) (Y :type Integer))
  (returns (New_Index :type Integer) (Real :type Boolean))
  (bind (_x_coordinate _y_coordinate) (`self.Split_Index` Index X Y))
  (bind _returnvalue (`self.Build_Index` _x_coordinate _y_coordinate)
    (:`Output`
      (return _returnvalue (and (`self.Check_New_Point` _x_coordinate) (`self.Check_New_Point` _y_coordinate))))))

(fn `Queen Component`
  (params (`Move priority` :type Boolean) (Checker :type "/Game/Blueprint/BP_Checker Object Reference"))
  (locals (`Next Point` :type Integer) (Finded :type Boolean))
  (bind _output (`|GetArrayItem` (`self.Field`) (`local.Next Point`)))
  (bind (_x_coordinate _y_coordinate) (`self.Split_Index` (`local.Next Point`) (`self.buf_X`) (`self.buf_Y`)))
  (bind (_x_coordinate_2 _y_coordinate_2) (`self.Split_Index` (`local.Next Point`) (`self.buf_X`) (`self.buf_Y`)))
  (for _index (range 4)
    (set `local.Next Point` (`/Game/Blueprint/BP_Checker.Posithion` Checker))
    (set `local.Finded` false)
    (if (`self.Multiplicity2` _index)
      (`self.Change_Buf_Variables` :!label _label
        (:`Output`
          (while (and (and (`self.Check_New_Point` _x_coordinate) (`self.Check_New_Point` _y_coordinate)) (not (`local.Finded`)))
            (bind _returnvalue (`self.Build_Index` _x_coordinate_2 _y_coordinate_2)
              (:`Output`
                (set `local.Next Point` _returnvalue)
                (if (`local.Move priority`)
                  (`/Engine/EditorBlueprintResources/StandardMacros.IsValid` _output
                    (:`Is Valid`
                      (if (`self.Is_Enemy` (`local.Checker`) _output)
                        (bind (_new_index _real) (`self.New Point` (`local.Next Point`) (`self.buf_X`) (`self.buf_Y`)))
                        (if _real
                          (`/Engine/EditorBlueprintResources/StandardMacros.IsValid` (`|GetArrayItem` (`self.Field`) _new_index)
                            (:`Is Valid`
                              _)
                            (:`Is Not Valid`
                              (`KismetArrayLibrary.Array_Add` (`/Game/Blueprint/BP_Checker.PosibleWays` (`local.Checker`)) _new_index)))
                          (set `local.Finded` true)))))
                  (else
                    (`/Engine/EditorBlueprintResources/StandardMacros.IsValid` _output
                      (:`Is Valid`
                        (set `local.Finded` true))
                      (:`Is Not Valid`
                        (`KismetArrayLibrary.Array_Add` (`/Game/Blueprint/BP_Checker.PosibleWays` (`local.Checker`)) (`local.Next Point`)))))))))))
      (else
        (goto _label :!via `False`)))))

(fn `Queen Ways`
  (params (Checker :type "/Game/Blueprint/BP_Checker Object Reference"))
  (bind _checker (`local.Checker`))
  (bind _probably_streak (`self.Probably Streak`))
  (`|ExecutionSequence`
    (:`then_0`
      (`self.Queen Component` true Checker))
    (:`then_1`
      (if (== (`KismetArrayLibrary.Array_Length` (`/Game/Blueprint/BP_Checker.PosibleWays` Checker)) 0)
        (if _probably_streak
          (set `self.Probably Streak` false)
          (set `/Game/Blueprint/BP_Checker.Streak` false _checker)
          (else
            (`self.Queen Component` false _checker)))
        (elif (not _probably_streak)
          (set `/Game/Blueprint/BP_Checker.Attack` true (`local.Checker`))
          (set `self.Under Attack` true))))))

(fn `Remove Checker`
  (bind (_x _y) (`self.Checker_Coordinate`))
  (bind _ref_checker (`self.Ref_Checker`))
  (bind _field (`self.Field`))
  (bind _ref_checker_2 (`self.Ref_Checker`))
  (bind _clicked_point (`self.Clicked_Point`))
  (bind _ref_checker_3 (`self.Ref_Checker`))
  (bind _ref_checker_4 (`self.Ref_Checker`))
  (bind _posithion (`/Game/Blueprint/BP_Checker.Posithion` _ref_checker_2))
  (`self.K2_SetActorLocation` (`self.Ref_Checker`) (`KismetMathLibrary.MakeVector` _x _y 32.0) false false)
  (`GameplayStatics.PlaySoundAtLocation` "/Game/Audio/S_Move.S_Move" (`self.K2_GetActorLocation`) (struct) 1.0 1.0 0.0 null null null)
  (if (`self.Become a Queen` (`self.Clicked_Point`))
    (`self.Set Queen` _ref_checker_2))
  (`KismetArrayLibrary.Array_Set` _field _clicked_point _ref_checker_2) ; Remove Checker to new Index
  (`KismetArrayLibrary.Array_Set` _field _posithion) ; Make null ref on old index
  (if (`/Game/Blueprint/BP_Checker.Attack` _ref_checker_4)
    (bind _killed_posithion (`self.Killed Posithion` _clicked_point _posithion))
    (`/Game/Blueprint/BP_Checker.Kill` _ref_checker_4 _killed_posithion)
    (set `self.Probably Streak` true)
    (if (`self.Turn Walk`)
      (`/Engine/EditorBlueprintResources/StandardMacros.IncrementInt` (`self.White Kills`)
        (:`  `
          _))
      (else
        (`/Engine/EditorBlueprintResources/StandardMacros.IncrementInt` (`self.Black Kills`)
          (:`  `
            _))))
    (`self.Update Text`)
    (set `/Game/Blueprint/BP_Checker.Posithion` (`self.Clicked_Point`) _ref_checker_3)
    (`KismetArrayLibrary.Array_Clear` (`/Game/Blueprint/BP_Checker.PosibleWays` _ref_checker_3))
    (if (`/Game/Blueprint/BP_Checker.Is Queen` (`self.Ref_Checker`))
      (`self.Queen Ways` _ref_checker)
      (else
        (`self.Add Point` _ref_checker)))
    (else
      (set `/Game/Blueprint/BP_Checker.Posithion` (`self.Clicked_Point`) (`self.Ref_Checker`)))))

(fn `Reset Checkers`
  (params (Desk :type "/Game/Blueprint/BP_Desk Object Reference"))
  (set `self.IsClick` false)
  (for _array_element (`self.Field`)
    (`/Engine/EditorBlueprintResources/StandardMacros.IsValid` _array_element
      (:`Is Valid`
        (set `/Game/Blueprint/BP_Checker.Clicked` false _array_element)
        (set `/Game/Blueprint/BP_Checker.Attack` false _array_element)
        (`/Game/Blueprint/BP_Checker.Refresh_Material` _array_element (`/Game/Blueprint/BP_Checker.StaticMesh` _array_element) (`/Game/Blueprint/BP_Checker.SIde(color)` _array_element))
        (`KismetArrayLibrary.Array_Clear` (`/Game/Blueprint/BP_Checker.PosibleWays` _array_element))))))

(fn `Set Clicked Checker`
  (params (Index :type Integer))
  (bind _output (`|GetArrayItem` (`self.Field`) Index))
  (`/Engine/EditorBlueprintResources/StandardMacros.IsValid` _output
    (:`Is Valid`
      (if (`/Game/Blueprint/BP_Checker.Clicked` _output)
        (set `self.Ref_Checker` _output)))))

(fn `Set Clicked Point`
  (params (Index :type Integer))
  (bind _returnvalue (`self.Build_Index` (`self.X`) (`self.Y`))
    (:`Output`
      (if (== _returnvalue Index)
        (set `self.Clicked_Point` _returnvalue)))))

(fn `Set Input Coordinates`
  (bind (_returnvalue_x _returnvalue_y) (`KismetMathLibrary.BreakVector` (/ (`.Location` (`GameplayStatics.BreakHitResult` (`PlayerController.GetHitResultUnderCursorByChannel` (`GameplayStatics.GetPlayerController` 0) "TraceTypeQuery1" true))) (50.0 50.0 1.0))))
  (set `self.X` (`KismetMathLibrary.FTrunc` _returnvalue_x))
  (set `self.Y` (`KismetMathLibrary.FTrunc` _returnvalue_y)))

(fn `Set Queen`
  (params (Checker :type "/Game/Blueprint/BP_Checker Object Reference"))
  (bind _staticmesh (`/Game/Blueprint/BP_Checker.StaticMesh` Checker))
  (set `/Game/Blueprint/BP_Checker.Is Queen` true Checker)
  (`StaticMeshComponent.SetStaticMesh` _staticmesh "/Game/Mesh/CheckerQueen.CheckerQueen")
  (`SceneComponent.K2_AddLocalRotation` _staticmesh (struct :`Yaw` 90.0) false false)
  (`GameplayStatics.PlaySoundAtLocation` "/Game/Audio/BecomeQueen.BecomeQueen" (`self.K2_GetActorLocation` Checker) (struct) 1.0 1.0 0.0 null null null))

(fn `Set Winner`
  (if (== (`self.White Kills`) 12)
    (set `self.Win` "White")
    (else
      (set `self.Win` "Black"))))

(fn `Update Text`
  (`/Engine/EditorBlueprintResources/StandardMacros.IsValid` (`self.Ref_Checker`)
    (:`Is Valid`
      (if (`self.Turn Walk`)
        (`TextBlock.SetText` (`/Game/Blueprint/WBP_HUD.KIlledCountW` (`self.Ref_HUD`)) (`KismetTextLibrary.Conv_IntToText` (`self.White Kills`)))
        (else
          (`TextBlock.SetText` (`/Game/Blueprint/WBP_HUD.KIlledCountB` (`self.Ref_HUD`)) (`KismetTextLibrary.Conv_IntToText` (`self.Black Kills`))))))))

(fn `UserConstructionScript`)