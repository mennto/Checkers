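; BP_Checker is a clickable checker piece that works with a board actor (RefDesk).
; Cursor hover switches to a hand; clicking selects the piece with a sound and yellow highlight, then asks the desk to identify moves, or resets checkers if a selection exists.
; Clicks are ignored while the desk's ProbablyStreak is set.
; Helper functions restore white or black material by side and destroy a captured piece, clearing its Field slot.
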(event `self.StaticMesh.OnBeginCursorOver`
  (params (TouchedComponent :type "PrimitiveComponent Object Reference"))
  (set `PlayerController.CurrentMouseCursor` "Hand" (`GameplayStatics.GetPlayerController` 0)))

(event `self.StaticMesh.OnEndCursorOver`
  (params (TouchedComponent :type "PrimitiveComponent Object Reference"))
  (set `PlayerController.CurrentMouseCursor` "Default" (`GameplayStatics.GetPlayerController` 0)))

(event `self.StaticMesh.OnClicked`
  (params (TouchedComponent :type "PrimitiveComponent Object Reference") (ButtonPressed :type "Key Structure"))
  (bind _ref_desk (`self.Ref_Desk`))
  (bind _ref_desk_2 (`self.Ref_Desk`))
  (if (`/Game/Blueprint/BP_Desk.Probably Streak` (`self.Ref_Desk`))
    _
    (elif (`/Game/Blueprint/BP_Desk.IsClick` _ref_desk_2)
      (`/Game/Blueprint/BP_Desk.Reset Checkers` _ref_desk_2 _ref_desk_2)
      (else
        (`GameplayStatics.PlaySoundAtLocation` "/Game/Audio/S_Touch.S_Touch" (`self.K2_GetActorLocation`) (struct) 1.0 1.0 0.0 null null null)
        (`PrimitiveComponent.SetMaterial` (`self.StaticMesh`) 0 "/Game/Material/M_yellow.M_yellow")
        (set `self.Clicked` true)
        (set `/Game/Blueprint/BP_Desk.IsClick` true _ref_desk)
        (`/Game/Blueprint/BP_Desk.Identify Ways` _ref_desk)))))

(fn `Kill`
  (params (Coordinate :type Integer))
  (bind _field (`/Game/Blueprint/BP_Desk.Field` (`self.Ref_Desk`)))
  (bind _output (`|GetArrayItem` _field Coordinate))
  (`GameplayStatics.PlaySoundAtLocation` "/Game/Audio/S_Death.S_Death" (`self.K2_GetActorLocation` _output) (struct) 1.0 1.0 0.0 null null null)
  (`self.K2_DestroyActor` _output)
  (`KismetArrayLibrary.Array_Set` _field Coordinate))

(fn `Refresh_Material`
  (params (Static_Mesh :type "PrimitiveComponent Object Reference") (Side :type Boolean))
  (if Side
    (`PrimitiveComponent.SetMaterial` Static_Mesh 0 "/Game/Material/M_white.M_white")
    (else
      (`PrimitiveComponent.SetMaterial` Static_Mesh 0 "/Game/Material/M_black.M_black"))))

(fn `UserConstructionScript`)